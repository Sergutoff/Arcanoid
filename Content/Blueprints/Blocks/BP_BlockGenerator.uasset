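; BP_BlockGenerator is an actor that spawns a flat grid of BP_Block_V0 blocks when play begins.
; Nested loops over Y and X place each block at the generator's location, offset in the XY plane by the loop indices times Padding.
; Blocks always spawn regardless of collision, and the construction script is empty, so the grid is built only at runtime.
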(event `self.ReceiveBeginPlay`
  (for _index (range (+ (`self.Y`) 1))
    (for _index_2 (range (+ (`self.X`) 1))
      (`|SpawnActorFromClass` "/Game/Blueprints/Blocks/BP_Block_V0.BP_Block_V0_C" (`KismetMathLibrary.MakeTransform` (+ (`self.K2_GetActorLocation`) (`KismetMathLibrary.MakeVector` (`KismetMathLibrary.Conv_IntToDouble` (* _index_2 (`self.Padding`))) (`KismetMathLibrary.Conv_IntToDouble` (* _index (`self.Padding`)))))) "AlwaysSpawn" "OverrideRootScale" null null))))

(fn `UserConstructionScript`)