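; BP_Block_V3 is a moving block that awards score to the GameInstance when it hits BP_Pawn, then destroys itself with a catch sound.
; It moves every Tick by a swept offset along its direction and speed.
; Hits from balls or BP_Block05, or overlapping a KillZVolume, mark it dead and swap its material.
; While dead, its cube scales up exponentially per frame until past a threshold, then it is destroyed with a death sound.
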(event `self.ReceiveActorBeginOverlap`
  (params (OtherActor :type "Actor Object Reference"))
  (cast `KillZVolume` OtherActor)
  (set `self.Dead` true)
  (`PrimitiveComponent.SetMaterial` (`self.Cube`) 0 "/Game/Material/Material_Instances/Cube_V3Dead_Mat_inst.Cube_V3Dead_Mat_inst"))

(event `self.ReceiveTick`
  (params (DeltaSeconds :type "Float (single-precision)"))
  (`|ExecutionSequence`
    (:`then_0`
      ;[1 1 1] Эффект разрушения
      (if (`self.Dead`)
        (bind _output_get (set `self.Size` (* (`self.Size`) 1.5)))
        (`SceneComponent.SetWorldScale3D` (`self.Cube`) (`KismetMathLibrary.Conv_DoubleToVector` _output_get))
        (if (> _output_get 1.0)
          (`self.K2_DestroyActor`)
          (`GameplayStatics.PlaySound2D` "/Game/Audio/Wawes/BlockDead.BlockDead" 1.0 1.0 0.0 null null))))
    (:`then_1`
      (`self.K2_AddActorWorldOffset` (* (* (`self.Dierection`) (`self.Speed`)) DeltaSeconds) true))))

(event `self.ReceiveHit`
  (params (MyComp :type "PrimitiveComponent Object Reference") (Other :type "Actor Object Reference") (OtherComp :type "PrimitiveComponent Object Reference") (bSelfMoved :type Boolean) (HitLocation :type "Vector Structure") (HitNormal :type "Vector Structure") (NormalImpulse :type "Vector Structure") (Hit :type "HitResult Structure (by ref)"))
  (bind _arcanoid_game_instance (`/Game/Blueprints/BP_FunctionLibrary.Cast to GameInstance`))
  (`|ExecutionSequence`
    (:`then_0`
      (cast `/Game/Blueprints/Character/BP_Pawn` Other)
      (`self.K2_DestroyActor`)
      (`GameplayStatics.PlaySound2D` "/Game/Audio/Wawes/BlockCatch.BlockCatch" 1.0 1.0 0.0 null null)
      (set `/Game/Blueprints/Arcanoid_GameInstance.Score` (+ (`/Game/Blueprints/Arcanoid_GameInstance.Score` _arcanoid_game_instance) 10) _arcanoid_game_instance))
    (:`then_1`
      (cast `/Game/Blueprints/Balls/BP_Ball` Other)
      (set `self.Dead` true :!label _label)
      (`PrimitiveComponent.SetMaterial` (`self.Cube`) 0 "/Game/Material/Material_Instances/Cube_V3Dead_Mat_inst.Cube_V3Dead_Mat_inst"))
    (:`then_2`
      (cast `/Game/Blueprints/Balls/BP_Ball_01` Other)
      (goto _label))
    (:`then_3`
      (cast `/Game/Blueprints/Blocks/BP_Block05` Other)
      (goto _label))))

(fn `UserConstructionScript`)