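; BP_Block_V0 is a two-hit block that scores points and can turn into a variant block when struck by a ball.
; The first hit randomly flags a V1–V7 variant, with V6 and V7 gated by level, and marks the cube through custom depth stencil.
; A later hit destroys it after a short delay, adds score to the GameInstance (more for BP_Ball_01 than BP_Ball) and spawns any flagged variant.
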(event `self.ReceiveHit`
  (params (MyComp :type "PrimitiveComponent Object Reference") (Other :type "Actor Object Reference") (OtherComp :type "PrimitiveComponent Object Reference") (bSelfMoved :type Boolean) (HitLocation :type "Vector Structure") (HitNormal :type "Vector Structure") (NormalImpulse :type "Vector Structure") (Hit :type "HitResult Structure (by ref)"))
  (bind _arcanoid_game_instance (`/Game/Blueprints/BP_FunctionLibrary.Cast to GameInstance`))
  (bind _returnvalue (`self.K2_GetActorLocation`))
  (bind _cube (`self.Cube`))
  (`|ExecutionSequence`
    (:`then_0`
      (cast `/Game/Blueprints/Balls/BP_Ball_01` Other)
      (if (`self.bWasHit`)
        (`KismetSystemLibrary.Delay` 0.2)
        (`self.K2_DestroyActor`)
        (`|ExecutionSequence`
          (:`then_0`
            (set `/Game/Blueprints/Arcanoid_GameInstance.Score` (+ (`/Game/Blueprints/Arcanoid_GameInstance.Score` _arcanoid_game_instance) 3) _arcanoid_game_instance))
          (:`then_1`
            (if (`self.bWasHitV7`) :!label _label
              (`|SpawnActorFromClass` "/Game/Blueprints/Blocks/BP_Block_V7.BP_Block_V7_C" (`KismetMathLibrary.MakeTransform` _returnvalue) "Undefined" "OverrideRootScale" null null)))
          (:`then_2`
            (if (`self.bWasHitV6`) :!label _label_2
              (`|SpawnActorFromClass` "/Game/Blueprints/Blocks/BP_Block_V6.BP_Block_V6_C" (`KismetMathLibrary.MakeTransform` _returnvalue) "Undefined" "OverrideRootScale" null null)))
          (:`then_3`
            (if (`self.bWasHit V5`) :!label _label_3
              (`|SpawnActorFromClass` "/Game/Blueprints/Blocks/BP_Block_V5.BP_Block_V5_C" (`KismetMathLibrary.MakeTransform` _returnvalue) "Undefined" "OverrideRootScale" null null)))
          (:`then_4`
            (if (`self.bWasHit V4`) :!label _label_4
              (`|SpawnActorFromClass` "/Game/Blueprints/Blocks/BP_Block_V4.BP_Block_V4_C" (`KismetMathLibrary.MakeTransform` _returnvalue) "Undefined" "OverrideRootScale" null null)))
          (:`then_5`
            (if (`self.bWasHit V3`) :!label _label_5
              (`|SpawnActorFromClass` "/Game/Blueprints/Blocks/BP_Block_V3.BP_Block_V3_C" (`KismetMathLibrary.MakeTransform` _returnvalue) "Undefined" "OverrideRootScale" null null)))
          (:`then_6`
            (if (`self.bWasHit V2`) :!label _label_6
              (`|SpawnActorFromClass` "/Game/Blueprints/Blocks/BP_Block_V2.BP_Block_V2_C" (`KismetMathLibrary.MakeTransform` _returnvalue) "Undefined" "OverrideRootScale" null null)))
          (:`then_7`
            (if (`self.bWasHit V1`) :!label _label_7
              (`|SpawnActorFromClass` "/Game/Blueprints/Blocks/BP_Block_V1.BP_Block_V1_C" (`KismetMathLibrary.MakeTransform` _returnvalue) "Undefined" "OverrideRootScale" null null))))
        (else
          (if (<= (`KismetMathLibrary.RandomFloat`) 0.3) :!label _label_8
            (if (`KismetMathLibrary.RandomBool`)
              (if (<= (`KismetMathLibrary.RandomFloat`) 0.7)
                (if (<= (`KismetMathLibrary.RandomFloat`) 0.3)
                  (`PrimitiveComponent.SetCustomDepthStencilValue` _cube 5)
                  (set `self.bWasHit` true)
                  (set `self.bWasHit V5` true)
                  (else
                    (`PrimitiveComponent.SetCustomDepthStencilValue` _cube 4)
                    (set `self.bWasHit` true)
                    (set `self.bWasHit V4` true)))
                (else
                  (`PrimitiveComponent.SetCustomDepthStencilValue` _cube 3)
                  (set `self.bWasHit` true)
                  (set `self.bWasHit V3` true)))
              (else
                (`PrimitiveComponent.SetCustomDepthStencilValue` _cube 2)
                (set `self.bWasHit` true)
                (set `self.bWasHit V2` true)))
            (elif (<= (`KismetMathLibrary.RandomFloat`) 0.3)
              (if (`KismetMathLibrary.RandomBool`)
                (if (== (`/Game/Blueprints/Arcanoid_GameInstance.Level_№` (`/Game/Blueprints/BP_FunctionLibrary.Cast to GameInstance`)) 3)
                  (`PrimitiveComponent.SetCustomDepthStencilValue` _cube 7)
                  (set `self.bWasHit` true)
                  (set `self.bWasHitV7` true)
                  (else
                    (`PrimitiveComponent.SetCustomDepthStencilValue` _cube 1 :!label _label_9)
                    (set `self.bWasHit` true)
                    (if (<= (`KismetMathLibrary.RandomFloat`) 0.2)
                      (set `self.bWasHit V1` true))))
                (elif (>= (`/Game/Blueprints/Arcanoid_GameInstance.Level_№` (`/Game/Blueprints/BP_FunctionLibrary.Cast to GameInstance`)) 2)
                  (`PrimitiveComponent.SetCustomDepthStencilValue` _cube 6)
                  (set `self.bWasHit` true)
                  (set `self.bWasHitV6` true)
                  (else
                    (goto _label_9))))
              (else
                (goto _label_9)))))))
    (:`then_1`
      (cast `/Game/Blueprints/Balls/BP_Ball` Other)
      (if (`self.bWasHit`)
        (`KismetSystemLibrary.Delay` 0.2)
        (`self.K2_DestroyActor`)
        (`|ExecutionSequence`
          (:`then_0`
            (`/Engine/EditorBlueprintResources/StandardMacros.IncrementInt` (`/Game/Blueprints/Arcanoid_GameInstance.Score` _arcanoid_game_instance)))
          (:`then_1`
            (goto _label))
          (:`then_2`
            (goto _label_2))
          (:`then_3`
            (goto _label_3))
          (:`then_4`
            (goto _label_4))
          (:`then_5`
            (goto _label_5))
          (:`then_6`
            (goto _label_6))
          (:`then_7`
            (goto _label_7)))
        (else
          (goto _label_8))))))

(fn `UserConstructionScript`)