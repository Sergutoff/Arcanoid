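; BP_Block05 is a block actor that spins its cube while sliding back and forth along the Y axis.
; Tick rotates the Cube in world space and moves the actor with a swept offset, both scaled by speed variables and delta time.
; A four-second Delay chained on Tick acts as a repeating timer that flips the movement direction between positive and negative Y.
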(event `self.ReceiveTick`
  (params (DeltaSeconds :type "Float (single-precision)"))
  (bind (_directionloc_x _directionloc_y) (`KismetMathLibrary.BreakVector` (`self.DirectionLoc`)))
  (`SceneComponent.K2_AddWorldRotation` (`self.Cube`) (* (* (`self.DierectionRot`) (`self.Speed_R`)) DeltaSeconds) false false)
  (`self.K2_AddActorWorldOffset` (* (* (`self.DirectionLoc`) (`self.Speed_L`)) DeltaSeconds) true)
  (`KismetSystemLibrary.Delay` 4.0)
  (if (> _directionloc_y 0.0)
    (set `self.DirectionLoc` (0.0 -100.0 0.0))
    (else
      (set `self.DirectionLoc` (0.0 100.0 0.0)))))

(fn `UserConstructionScript`)