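; Arkanoid game mode that runs the countdown, win/loss flow and special level effects.
; A looping timer counts remaining blocks and, at zero, opens the next level or game-over menu using game instance flags.
; Tick uses a Delay for the countdown and drives Material Parameter Collection outlines around the Playground sphere, with the Level 3 effect also flipping player direction.
; An optional frozen look adds snowfall and a timeline-animated dynamic post-process material.
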(event `Create Frozen and Snow`
  ;[1 1 1] Snow and Frozen
  (bind _returnvalue (`KismetMaterialLibrary.CreateDynamicMaterialInstance` "/Game/Material/Material_Instances/Frozen_Material_Inst.Frozen_Material_Inst"))
  (bind _output_get (set `self.Dynamic Post Process` _returnvalue))
  (bind _returnvalue_2 (`GameplayStatics.GetActorOfClass` "/Script/Engine.CameraActor"))
  (setmembers `PostProcessSettings` :`StructRef` (`CameraComponent.PostProcessSettings` (`CameraActor.CameraComponent` _returnvalue_2)) :`WeightedBlendables` (make `WeightedBlendables` (`|MakeArray` (make `WeightedBlendable` 1.0 _output_get))))
  (`self.Start Frozen and Snow PostProcess`))

(event `Start Frozen and Snow PostProcess`
  ;[1 1 1] Snow and Frozen
  (`|ExecutionSequence`
    (:`then_0`
      (`GameplayStatics.SpawnEmitterAtLocation` (`self.Snowfall`) (2000.0 0.0 -1000.0) (struct :`Pitch` -90.0) (5.0 5.0 5.0)))
    (:`then_1`
      (bind (_direction _newtrack_0) (`Timeline|Timeline_2`)
        (:`Update`
          (`MaterialInstanceDynamic.SetScalarParameterValue` (`self.Dynamic Post Process`) "Density" _newtrack_0))))))

(event `self.ReceiveBeginPlay`
  (`|ExecutionSequence`
    (:`then_0`
      (if (`/Game/Blueprints/Arcanoid_GameInstance.SnowFrozen` (`/Game/Blueprints/BP_FunctionLibrary.Cast to GameInstance`))
        (`self.Create Frozen and Snow`)))
    (:`then_1`
      (`KismetSystemLibrary.K2_SetTimerDelegate` (delegate `BlockCount`) 0.1 true))))

(event `BlockCount`
  (bind _arcanoid_game_instance (`/Game/Blueprints/BP_FunctionLibrary.Cast to GameInstance`))
  (bind _outactors (`GameplayStatics.GetAllActorsOfClass` "/Game/Blueprints/Blocks/BP_Block_V0.BP_Block_V0_C"))
  (bind _output_get (set `self.CountBlock` (`KismetArrayLibrary.Array_Length` _outactors)))
  (if (== _output_get 0)
    (set `self.Win?` true)
    (set `/Game/Blueprints/Arcanoid_GameInstance.Win?` true _arcanoid_game_instance)
    (`/Game/Blueprints/Arcanoid_GameInstance.Stored Levels` _arcanoid_game_instance)
    (`KismetSystemLibrary.Delay` 0.5)
    (if (== (`/Game/Blueprints/Arcanoid_GameInstance.Level_Index` _arcanoid_game_instance) 3)
      (if (`/Game/Blueprints/Arcanoid_GameInstance.L_02?` _arcanoid_game_instance)
        (`GameplayStatics.OpenLevel` "Level_02")
        (set `/Game/Blueprints/Arcanoid_GameInstance.Level_№` 2 _arcanoid_game_instance)
        (set `/Game/Blueprints/Arcanoid_GameInstance.L_02?` false _arcanoid_game_instance)
        (elif (`/Game/Blueprints/Arcanoid_GameInstance.L_03?` _arcanoid_game_instance)
          (`GameplayStatics.OpenLevel` "Level_03")
          (set `/Game/Blueprints/Arcanoid_GameInstance.Level_№` 3 _arcanoid_game_instance)
          (set `/Game/Blueprints/Arcanoid_GameInstance.L_03?` false _arcanoid_game_instance)
          (else
            (`GameplayStatics.OpenLevel` "GameOver_Menu" :!label _label)
            (set `/Game/Blueprints/Arcanoid_GameInstance.L_02?` true _arcanoid_game_instance)
            (set `/Game/Blueprints/Arcanoid_GameInstance.L_03?` true _arcanoid_game_instance))))
      (else
        (goto _label)))))

(event `self.ReceiveTick`
  (params (DeltaSeconds :type "Float (single-precision)"))
  (bind _bp_pawn (`/Game/Blueprints/BP_FunctionLibrary.Cast to Player Pawn`))
  (bind _arcanoid_game_instance (`/Game/Blueprints/BP_FunctionLibrary.Cast to GameInstance`))
  (bind _seconds (`self.Seconds`))
  (bind _minutes (`self.Minutes`))
  (`|ExecutionSequence`
    (:`then_0`
      ;[1 1 1] Countdown Timer
      (`KismetSystemLibrary.Delay` 1.0)
      (if (== _seconds 0)
        (if (== _minutes 0)
          (set `self.TimeOver?` true)
          (set `/Game/Blueprints/Arcanoid_GameInstance.TimeOver?` true (`/Game/Blueprints/BP_FunctionLibrary.Cast to GameInstance`))
          (`GameplayStatics.PlaySound2D` "/Game/Audio/Wawes/TimeOver.TimeOver" 1.0 1.0 0.0 null null)
          (`KismetSystemLibrary.Delay` 0.7)
          (`GameplayStatics.OpenLevel` "GameOver_Menu")
          (set `/Game/Blueprints/Arcanoid_GameInstance.L_02?` true _arcanoid_game_instance)
          (set `/Game/Blueprints/Arcanoid_GameInstance.L_03?` true _arcanoid_game_instance)
          (else
            (set `self.Seconds` 59)
            (set `self.Minutes` (- _minutes 1))))
        (else
          (set `self.Seconds` (- _seconds 1))
          ;[1 1 1] Отсчёт времени последних 10 сек.
          (if (== (`self.Minutes`) 0)
            (if (<= (`self.Seconds`) 10)
              (`GameplayStatics.PlaySound2D` "/Game/Audio/Wawes/Last_10_sec.Last_10_sec" 1.0 1.0 0.0 null null))))))
    (:`then_1`
      (if (`self.Outlines_L2`)
        (`KismetMaterialLibrary.SetVectorParameterValue` "/Game/Material/Outlines_Material/PC_L2_OutlineData.PC_L2_OutlineData" "Location" (`KismetMathLibrary.Conv_VectorToLinearColor` (`SceneComponent.K2_GetComponentLocation` (`/Game/Blueprints/BP_Playground.Sphere` (`/Game/Blueprints/BP_FunctionLibrary.Cast to Playground`)))))
        (if (`self.CatchBlock_V6`)
          (set `self.Outlines_L2` false)
          (set `self.CatchBlock_V6` false)
          (bind (_direction _newtrack_0) (`Timeline|Timeline_0` :!via `Reverse` :!label _label_2)
            (:`Update`
              (`KismetMaterialLibrary.SetScalarParameterValue` "/Game/Material/Outlines_Material/PC_L2_OutlineData.PC_L2_OutlineData" "Radius" _newtrack_0)))
          (else
            (goto _label_2)))))
    (:`then_2`
      (if (`self.Outlines_L3`)
        (`KismetMaterialLibrary.SetVectorParameterValue` "/Game/Material/Outlines_Material/PC_L3_OutlineData.PC_L3_OutlineData" "Location" (`KismetMathLibrary.Conv_VectorToLinearColor` (`SceneComponent.K2_GetComponentLocation` (`/Game/Blueprints/BP_Playground.Sphere` (`/Game/Blueprints/BP_FunctionLibrary.Cast to Playground`)))))
        (if (`self.CatchBlock_V7`)
          (set `/Game/Blueprints/Character/BP_Pawn.Direction` 1 _bp_pawn)
          (set `self.Outlines_L3` false)
          (set `self.CatchBlock_V7` false)
          (bind (_direction_2 _newtrack_0_2) (`Timeline|Timeline_1` :!via `Reverse` :!label _label_3)
            (:`Update`
              (`KismetMaterialLibrary.SetScalarParameterValue` "/Game/Material/Outlines_Material/PC_L3_OutlineData.PC_L3_OutlineData" "Radius" _newtrack_0_2)))
          (else
            (set `/Game/Blueprints/Character/BP_Pawn.Direction` -1 _bp_pawn)
            (goto _label_3)))))))

(fn `UserConstructionScript`)