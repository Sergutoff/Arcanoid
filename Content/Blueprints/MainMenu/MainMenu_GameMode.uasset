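; Main menu game mode that drives a frozen-screen post-process effect and snowfall.
; On BeginPlay it puts a dynamic frost material on the CameraActor's post-process settings, then restores its Density and spawns snow if the game instance's SnowFrozen flag is set.
; Start and Close events play or reverse a timeline that animates Density and saves it to the game instance, while spawning or removing the snow emitters.
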(event `self.ReceiveBeginPlay`
  (bind _arcanoid_game_instance (`/Game/Blueprints/BP_FunctionLibrary.Cast to GameInstance`))
  (bind _dynamic_post_process (`self.Dynamic Post Process`))
  (`self.Create Frozen and Snow`)
  (if (`/Game/Blueprints/Arcanoid_GameInstance.SnowFrozen` _arcanoid_game_instance)
    (`MaterialInstanceDynamic.SetScalarParameterValue` _dynamic_post_process "Density" (`/Game/Blueprints/Arcanoid_GameInstance.Density` _arcanoid_game_instance))
    (bind _returnvalue (`GameplayStatics.SpawnEmitterAtLocation` (`self.Snowfall`) (0.0 1800.0 2000.0)))
    (else
      (`MaterialInstanceDynamic.SetScalarParameterValue` _dynamic_post_process "Density" 20.0))))

(event `Create Frozen and Snow`
  ;[1 1 1] Snow and Frozen
  (bind _returnvalue (`KismetMaterialLibrary.CreateDynamicMaterialInstance` "/Game/Material/Material_Instances/Frozen_Material_Inst.Frozen_Material_Inst"))
  (bind _output_get (set `self.Dynamic Post Process` _returnvalue))
  (bind _returnvalue_2 (`GameplayStatics.GetActorOfClass` "/Script/Engine.CameraActor"))
  (setmembers `PostProcessSettings` :`StructRef` (`CameraComponent.PostProcessSettings` (`CameraActor.CameraComponent` _returnvalue_2)) :`WeightedBlendables` (make `WeightedBlendables` (`|MakeArray` (make `WeightedBlendable` 1.0 _output_get)))))

(event `Start Frozen and Snow PostProcess`
  ;[1 1 1] Snow and Frozen
  (`|ExecutionSequence`
    (:`then_0`
      (bind _returnvalue (`GameplayStatics.SpawnEmitterAtLocation` (`self.Snowfall`) (0.0 1800.0 2000.0))))
    (:`then_1`
      (bind (_direction _newtrack_0) (`Timeline|Timeline_0` :!label _label)
        (:`Update`
          (bind _output_get (set `/Game/Blueprints/Arcanoid_GameInstance.Density` _newtrack_0 (`/Game/Blueprints/BP_FunctionLibrary.Cast to GameInstance`)))
          (`MaterialInstanceDynamic.SetScalarParameterValue` (`self.Dynamic Post Process`) "Density" _output_get))))))

(event `Close Frozen and Snow PostProcess`
  ;[1 1 1] Snow and Frozen
  (`|ExecutionSequence`
    (:`then_0`
      (goto _label :!via `Reverse`))
    (:`then_1`
      (`KismetSystemLibrary.Delay` 2.0)
      (`ActorComponent.Deactivate` (stale `Start Frozen and Snow PostProcess` _returnvalue)))
    (:`then_2`
      (`ActorComponent.K2_DestroyComponent` (stale `self.ReceiveBeginPlay` _returnvalue)))))

(fn `UserConstructionScript`)