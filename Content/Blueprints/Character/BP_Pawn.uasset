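; Player paddle pawn for an Arkanoid-style game, moving sideways with swept offsets and managing the ball and lives.
; BeginPlay spawns the ball, creates the HUD in UI-only input, checks the save and resets GameMode flags.
; Hits from block types trigger effects: extra ball, block removal, added life, GameMode minute increment or faster ball.
; The ball's OnDead event drives BallDead, which respawns it using a life or opens game over at zero.
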(event `InputAxis|MoveRight`
  (params (AxisValue :type "Float (single-precision)"))
  (bind _output_get (set `self.LastMoveDirection` (`KismetMathLibrary.MakeVector` 0.0 (* (`self.Direction`) (* AxisValue (`self.BP_PawnSpeed`) (`GameplayStatics.GetWorldDeltaSeconds`))))))
  (`self.K2_AddActorWorldOffset` _output_get true))

(event `self.ReceiveBeginPlay`
  (bind _arcanoid_game_mode (`/Game/Blueprints/BP_FunctionLibrary.Cast to Arcanoid GameMode`))
  (bind _returnvalue (`GameplayStatics.GetPlayerController` 0))
  (`|ExecutionSequence`
    (:`then_0`
      (`KismetSystemLibrary.Delay` 0.5)
      (`/Engine/EditorBlueprintResources/StandardMacros.IsValid` (`self.PlayingBall`)
        (:`Is Not Valid`
          (`self.SpawnBall`)
          (`GameplayStatics.PlaySound2D` "/Game/Audio/Wawes/SpawnBall_Sound.SpawnBall_Sound" 1.0 1.0 0.0 null null))))
    (:`then_1`
      (bind _returnvalue_2 (`|CreateWidget` "/Game/UI/Main_HUD.Main_HUD_C"))
      (bind _output_get (set `self.Main HUD` _returnvalue_2))
      (`UserWidget.AddToViewport` _output_get 0)
      (set `PlayerController.bShowMouseCursor` true _returnvalue)
      (`WidgetBlueprintLibrary.SetInputMode_UIOnlyEx` _returnvalue _output_get "LockInFullscreen"))
    (:`then_2`
      (`/Game/Blueprints/Arcanoid_GameInstance.CheckSave` (`/Game/Blueprints/BP_FunctionLibrary.Cast to GameInstance`)))
    (:`then_3`
      (set `/Game/Blueprints/Arcanoid_GameMode.Outlines_L2` false _arcanoid_game_mode)
      (set `/Game/Blueprints/Arcanoid_GameMode.Outlines_L3` false _arcanoid_game_mode)
      (set `/Game/Blueprints/Arcanoid_GameMode.CatchBlock_V6` false _arcanoid_game_mode)
      (set `/Game/Blueprints/Arcanoid_GameMode.CatchBlock_V7` false _arcanoid_game_mode))))

(event `self.ReceiveTick`
  (params (DeltaSeconds :type "Float (single-precision)")))

(event `self.ReceiveHit`
  (params (MyComp :type "PrimitiveComponent Object Reference") (Other :type "Actor Object Reference") (OtherComp :type "PrimitiveComponent Object Reference") (bSelfMoved :type Boolean) (HitLocation :type "Vector Structure") (HitNormal :type "Vector Structure") (NormalImpulse :type "Vector Structure") (Hit :type "HitResult Structure (by ref)"))
  (bind _playingball (`self.PlayingBall`))
  (bind _maxspeed (`/Game/Blueprints/Balls/BP_Ball.MaxSpeed` _playingball))
  (bind _returnvalue (+ (`/Game/Blueprints/Balls/BP_Ball.Speed` _playingball) (`/Game/Blueprints/Balls/BP_Ball.Increase` _playingball)))
  (`|ExecutionSequence`
    (:`then_0`
      (cast `/Game/Blueprints/Blocks/BP_Block_V4` Other)
      (`KismetSystemLibrary.Delay` 0.3)
      (`|SpawnActorFromClass` "/Game/Blueprints/Balls/BP_Ball_01.BP_Ball_01_C" (`KismetMathLibrary.MakeTransform` (`SceneComponent.K2_GetComponentLocation` (`self.Capsule1`))) "AdjustIfPossibleButAlwaysSpawn" "OverrideRootScale" null null))
    (:`then_1`
      (cast `/Game/Blueprints/Blocks/BP_Block_V2` Other)
      (`|ExecutionSequence`
        (:`then_0`
          (bind _outactors (`GameplayStatics.GetAllActorsOfClass` "/Game/Blueprints/Blocks/BP_4Blocks.BP_4Blocks_C"))
          (`self.K2_DestroyActor` _outactors))
        (:`then_1`
          (bind _outactors_2 (`GameplayStatics.GetAllActorsOfClass` "/Game/Blueprints/Blocks/BP_Block05.BP_Block05_C"))
          (`self.K2_DestroyActor` _outactors_2))))
    (:`then_2`
      (cast `/Game/Blueprints/Blocks/BP_Block_V3` Other)
      (bind _result (`/Engine/EditorBlueprintResources/StandardMacros.IncrementInt` (`self.Ball Count`))
        (:`  `
          (set `self.Ball Count` _result))))
    (:`then_3`
      (cast `/Game/Blueprints/Blocks/BP_Block_V5` Other)
      (bind _asarcanoid_game_mode (cast `/Game/Blueprints/Arcanoid_GameMode` (`GameplayStatics.GetGameMode`)))
      (bind _result_2 (`/Engine/EditorBlueprintResources/StandardMacros.IncrementInt` (`/Game/Blueprints/Arcanoid_GameMode.Minutes` _asarcanoid_game_mode))
        (:`  `
          (set `/Game/Blueprints/Arcanoid_GameMode.Minutes` _result_2 _asarcanoid_game_mode))))
    (:`then_4`
      (cast `/Game/Blueprints/Blocks/BP_Block_V1` Other)
      ;[1 1 1] Увеличение скорости шарика
      (`KismetSystemLibrary.Delay` 0.2)
      (`/Engine/EditorBlueprintResources/StandardMacros.IsValid` _playingball
        (:`Is Valid`
          (if (>= _returnvalue _maxspeed)
            (`/Engine/EditorBlueprintResources/StandardMacros.IsValid` _playingball
              (:`Is Valid`
                (set `/Game/Blueprints/Balls/BP_Ball.Speed` _maxspeed _playingball)
                (`KismetSystemLibrary.Delay` 0.2)
                (set `self.BallSpeed` 7)))
            (else
              (`/Engine/EditorBlueprintResources/StandardMacros.IsValid` _playingball
                (:`Is Valid`
                  (set `/Game/Blueprints/Balls/BP_Ball.Speed` _returnvalue _playingball)
                  (`KismetSystemLibrary.Delay` 0.2)
                  (set `self.BallSpeed` (+ (`self.BallSpeed`) 1)))))))))))

(event `SpawnBall`
  ;[1 1 1] Создание шариков
  (bind _returnvalue (`|SpawnActorFromClass` "/Game/Blueprints/Balls/BP_Ball.BP_Ball_C" (`KismetMathLibrary.MakeTransform` (`SceneComponent.K2_GetComponentLocation` (`self.Capsule`))) "AdjustIfPossibleButAlwaysSpawn" "OverrideRootScale" null null))
  (bind _output_get (set `self.PlayingBall` _returnvalue))
  (add `/Game/Blueprints/Balls/BP_Ball.OnDead` _output_get (delegate `BallDead`)))

(event `BallDead`
  (bind _arcanoid_game_instance (`/Game/Blueprints/BP_FunctionLibrary.Cast to GameInstance`))
  ;[1 1 1] Создание шариков
  (if (>= (`self.Ball Count`) (`self.Min Ball Count`))
    (`KismetSystemLibrary.Delay` 1.0)
    (`/Engine/EditorBlueprintResources/StandardMacros.IsValid` (`self.PlayingBall`)
      (:`Is Not Valid`
        (`self.SpawnBall`)
        (`GameplayStatics.PlaySound2D` "/Game/Audio/Wawes/SpawnBall_Sound.SpawnBall_Sound" 1.0 1.0 0.0 null null)
        (bind _result (`/Engine/EditorBlueprintResources/StandardMacros.DecrementInt` (`self.Ball Count`))
          (:`  `
            (set `self.Ball Count` _result)))))
    (elif (== (`self.Ball Count`) 0)
      (`KismetSystemLibrary.Delay` 0.3)
      (`GameplayStatics.PlaySound2D` "/Game/Audio/Wawes/EndPlay.EndPlay" 1.0 1.0 0.0 null null)
      (`GameplayStatics.OpenLevel` "GameOver_Menu")
      (set `/Game/Blueprints/Arcanoid_GameInstance.L_02?` true _arcanoid_game_instance)
      (set `/Game/Blueprints/Arcanoid_GameInstance.L_03?` true _arcanoid_game_instance))))

(fn `SpawnBall 2`)

(fn `UserConstructionScript`)