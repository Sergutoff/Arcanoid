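; BP_Ball is a bouncing ball actor that travels in a straight line until it overlaps a KillZVolume.
; Tick moves it with a swept offset, reflecting direction and playing a sound on blocking hits; pawn hits blend in the pawn's last move direction.
; Death fires OnDead, swaps material, sets the pawn's BallSpeed, then inflates the sphere until it is destroyed with a sound.
; Clamped speed increase and decrease logic exists but is never executed.
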(event `self.ReceiveBeginPlay`
  (set `self.Direction` (`KismetMathLibrary.Conv_RotatorToVector` (`self.K2_GetActorRotation`))))

(event `self.ReceiveActorBeginOverlap`
  (params (OtherActor :type "Actor Object Reference"))
  (cast `KillZVolume` OtherActor)
  (set `self.Dead` true)
  (`self.OnDead`)
  (`PrimitiveComponent.SetMaterial` (`self.Sphere`) 0 "/Game/Material/Material_Instances/BallDead_Mat_inst.BallDead_Mat_inst")
  (bind _asbp_pawn (cast `/Game/Blueprints/Character/BP_Pawn` (`GameplayStatics.GetPlayerPawn` 0)))
  (set `/Game/Blueprints/Character/BP_Pawn.BallSpeed` 1 _asbp_pawn))

(event `self.ReceiveTick`
  (params (DeltaSeconds :type "Float (single-precision)"))
  (`|ExecutionSequence`
    (:`then_0`
      ;[1 1 1] Эффект разрушения
      (if (`self.Dead`)
        (bind _output_get (set `self.BallSize` (* (`self.BallSize`) 1.5)))
        (`SceneComponent.SetWorldScale3D` (`self.Sphere`) (`KismetMathLibrary.Conv_DoubleToVector` _output_get))
        (if (> _output_get 3.0)
          (`self.K2_DestroyActor`)
          (`GameplayStatics.PlaySound2D` "/Game/Audio/Wawes/BallDead.BallDead" 1.0 1.0 0.0 null null))))
    (:`then_1`
      (bind _sweephitresult (`self.K2_AddActorWorldOffset` (* (* (`self.Direction`) (`self.Speed`)) DeltaSeconds) true))
      (bind (_bblockinghit _binitialoverlap _time _distance _location _impactpoint _normal) (`GameplayStatics.BreakHitResult` _sweephitresult))
      (if _bblockinghit
        (bind _output_get_2 (set `self.Direction` (`KismetMathLibrary.GetReflectionVector` (`self.Direction`) (`KismetMathLibrary.MakeVector` (.x _normal) (.y _normal)))))
        (`self.K2_SetActorRotation` (`KismetMathLibrary.Conv_VectorToRotator` _output_get_2))
        (`GameplayStatics.PlaySoundAtLocation` "/Game/Audio/Wawes/BallHit.BallHit" _output_get_2 (struct) 1.0 1.0 0.0 null null null)))))

(event `self.Sphere.OnComponentHit`
  (params (HitComponent :type "PrimitiveComponent Object Reference") (OtherActor :type "Actor Object Reference") (OtherComp :type "PrimitiveComponent Object Reference") (NormalImpulse :type "Vector Structure") (Hit :type "HitResult Structure (by ref)"))
  (bind _asbp_pawn (cast `/Game/Blueprints/Character/BP_Pawn` OtherActor))
  (set `self.Direction` (`KismetMathLibrary.Normal` (+ (`KismetMathLibrary.Normal` (`/Game/Blueprints/Character/BP_Pawn.LastMoveDirection` _asbp_pawn)) (`self.Direction`)))))

(fn `UserConstructionScript`)