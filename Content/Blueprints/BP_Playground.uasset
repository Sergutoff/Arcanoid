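; Playground actor whose two walls redirect balls that strike them.
; Each wall's hit event handles both BP_Ball and BP_Ball_01 with identical, duplicated logic.
; The normalized NewDirection vector is added to the ball's Direction when its X is non-negative, otherwise subtracted, and the result is renormalized.
; BeginPlay, overlap, Tick and the construction script are empty.
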(event `self.ReceiveBeginPlay`)

(event `self.ReceiveTick`
  (params (DeltaSeconds :type "Float (single-precision)")))

(event `self.Wall_1.OnComponentHit`
  (params (HitComponent :type "PrimitiveComponent Object Reference") (OtherActor :type "Actor Object Reference") (OtherComp :type "PrimitiveComponent Object Reference") (NormalImpulse :type "Vector Structure") (Hit :type "HitResult Structure (by ref)"))
  (bind _returnvalue (`KismetMathLibrary.Normal` (`self.NewDirection`)))
  (bind _returnvalue_2 (`KismetMathLibrary.Normal` (`self.NewDirection`)))
  (`|ExecutionSequence`
    (:`then_0`
      (bind _asbp_ball (cast `/Game/Blueprints/Balls/BP_Ball` OtherActor))
      (bind _direction_x (`KismetMathLibrary.BreakVector` (`/Game/Blueprints/Balls/BP_Ball.Direction` _asbp_ball)))
      (if (>= _direction_x 0.0)
        (bind _direction (`/Game/Blueprints/Balls/BP_Ball.Direction` _asbp_ball))
        (set `/Game/Blueprints/Balls/BP_Ball.Direction` (`KismetMathLibrary.Normal` (+ _direction _returnvalue)) _asbp_ball)
        (else
          (set `/Game/Blueprints/Balls/BP_Ball.Direction` (`KismetMathLibrary.Normal` (- _direction _returnvalue)) _asbp_ball))))
    (:`then_1`
      (bind _asbp_ball_01 (cast `/Game/Blueprints/Balls/BP_Ball_01` OtherActor))
      (bind _direction_x_2 (`KismetMathLibrary.BreakVector` (`/Game/Blueprints/Balls/BP_Ball_01.Direction` _asbp_ball_01)))
      (if (>= _direction_x_2 0.0)
        (bind _direction_2 (`/Game/Blueprints/Balls/BP_Ball_01.Direction` _asbp_ball_01))
        (set `/Game/Blueprints/Balls/BP_Ball_01.Direction` (`KismetMathLibrary.Normal` (+ _direction_2 _returnvalue_2)) _asbp_ball_01)
        (else
          (set `/Game/Blueprints/Balls/BP_Ball_01.Direction` (`KismetMathLibrary.Normal` (- _direction_2 _returnvalue_2)) _asbp_ball_01))))))

(event `self.Wall_2.OnComponentHit`
  (params (HitComponent :type "PrimitiveComponent Object Reference") (OtherActor :type "Actor Object Reference") (OtherComp :type "PrimitiveComponent Object Reference") (NormalImpulse :type "Vector Structure") (Hit :type "HitResult Structure (by ref)"))
  (bind _returnvalue (`KismetMathLibrary.Normal` (`self.NewDirection`)))
  (bind _returnvalue_2 (`KismetMathLibrary.Normal` (`self.NewDirection`)))
  (`|ExecutionSequence`
    (:`then_0`
      (bind _asbp_ball (cast `/Game/Blueprints/Balls/BP_Ball` OtherActor))
      (bind _direction_x (`KismetMathLibrary.BreakVector` (`/Game/Blueprints/Balls/BP_Ball.Direction` _asbp_ball)))
      (if (>= _direction_x 0.0)
        (bind _direction (`/Game/Blueprints/Balls/BP_Ball.Direction` _asbp_ball))
        (set `/Game/Blueprints/Balls/BP_Ball.Direction` (`KismetMathLibrary.Normal` (+ _direction _returnvalue_2)) _asbp_ball)
        (else
          (set `/Game/Blueprints/Balls/BP_Ball.Direction` (`KismetMathLibrary.Normal` (- _direction _returnvalue_2)) _asbp_ball))))
    (:`then_1`
      (bind _asbp_ball_01 (cast `/Game/Blueprints/Balls/BP_Ball_01` OtherActor))
      (bind _direction_x_2 (`KismetMathLibrary.BreakVector` (`/Game/Blueprints/Balls/BP_Ball_01.Direction` _asbp_ball_01)))
      (if (>= _direction_x_2 0.0)
        (bind _direction_2 (`/Game/Blueprints/Balls/BP_Ball_01.Direction` _asbp_ball_01))
        (set `/Game/Blueprints/Balls/BP_Ball_01.Direction` (`KismetMathLibrary.Normal` (+ _direction_2 _returnvalue)) _asbp_ball_01)
        (else
          (set `/Game/Blueprints/Balls/BP_Ball_01.Direction` (`KismetMathLibrary.Normal` (- _direction_2 _returnvalue)) _asbp_ball_01))))))

(fn `UserConstructionScript`)