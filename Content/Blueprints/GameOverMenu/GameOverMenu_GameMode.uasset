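; Game mode for the game over level that shows the Game Over menu through the game instance and plays a delayed victory sound on a win.
; When the game instance's SnowFrozen flag is set, it also applies a dynamic frozen post-process material to the level's camera actor.
; A snowfall emitter then spawns while a timeline drives the material's Density parameter.
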(event `Create Frozen and Snow`
  ;[1 1 1] Snow and Frozen
  (bind _returnvalue (`KismetMaterialLibrary.CreateDynamicMaterialInstance` "/Game/Material/Material_Instances/Frozen_Material_Inst.Frozen_Material_Inst"))
  (bind _output_get (set `self.Dynamic Post Process` _returnvalue))
  (bind _returnvalue_2 (`GameplayStatics.GetActorOfClass` "/Script/Engine.CameraActor"))
  (setmembers `PostProcessSettings` :`StructRef` (`CameraComponent.PostProcessSettings` (`CameraActor.CameraComponent` _returnvalue_2)) :`WeightedBlendables` (make `WeightedBlendables` (`|MakeArray` (make `WeightedBlendable` 1.0 _output_get))))
  (`self.Start Frozen and Snow PostProcess`))

(event `Start Frozen and Snow PostProcess`
  ;[1 1 1] Snow and Frozen
  (`|ExecutionSequence`
    (:`then_0`
      (`GameplayStatics.SpawnEmitterAtLocation` (`self.Snowfall`) (-3500.0 0.0 2000.0) (struct :`Pitch` 40.0) (2.0 2.0 2.0)))
    (:`then_1`
      (bind (_direction _newtrack_0) (`Timeline|Timeline_0`)
        (:`Update`
          (`MaterialInstanceDynamic.SetScalarParameterValue` (`self.Dynamic Post Process`) "Density" _newtrack_0))))))

(event `self.ReceiveBeginPlay`
  (bind _arcanoid_game_instance (`/Game/Blueprints/BP_FunctionLibrary.Cast to GameInstance`))
  (`|ExecutionSequence`
    (:`then_0`
      (if (`/Game/Blueprints/Arcanoid_GameInstance.SnowFrozen` (`/Game/Blueprints/BP_FunctionLibrary.Cast to GameInstance`))
        (`self.Create Frozen and Snow`)))
    (:`then_1`
      (`/Game/Blueprints/Arcanoid_GameInstance.Show GameOver Menu` _arcanoid_game_instance)
      (if (`/Game/Blueprints/Arcanoid_GameInstance.Win?` _arcanoid_game_instance)
        (`KismetSystemLibrary.Delay` 0.5)
        (`GameplayStatics.PlaySound2D` "/Game/Audio/Cue/Win__Cue.Win__Cue" 1.0 1.0 0.0 null null)))))

(fn `UserConstructionScript`)